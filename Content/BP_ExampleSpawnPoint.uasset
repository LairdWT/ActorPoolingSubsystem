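; Example spawn point that periodically spawns BP_ExampleActor through an actor pool rather than a plain spawn.
; BeginPlay starts a looping timer instead of using Tick, with initial delay variance to randomize when spawning starts.
; Each timer call runs ActorPoolSpawn's SpawnActor at a random horizontal offset below the spawn point, with spawn broadcasting enabled.
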(event Custom|Spawn%20Actor
  ;[1 1 1] Timer instead of tick! 0.25 second interval
  ;;[1 1 1] Event triggered by timer
  (Class|ActorPoolSpawnComponent|SpawnActor (Variables|Default|GetActorPoolSpawn) "/ActorPoolingSubsystem/BP_ExampleActor.BP_ExampleActor_C" (Math|Transform|MakeTransform (+ (Transformation|GetActorLocation self) (Math|Vector|MakeVector (Math|Random|RandomFloatinRange -5e+01 5e+01) (Math|Random|RandomFloatinRange -5e+01 5e+01) (Math|Random|RandomFloatinRange -2e+02 -5e+02)))) "AlwaysSpawn" true))

(event EventBeginPlay
  ;[1 1 1] Timer instead of tick! 0.25 second interval
  (Utilities|Time|SetTimerbyEvent (delegate Custom|Spawn%20Actor) 1.0 true 0.0 1.0))

(fn ConstructionScript)