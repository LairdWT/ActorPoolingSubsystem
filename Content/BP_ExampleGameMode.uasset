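; Example game mode that demonstrates setting up and listening to an actor pool through the ActorPoolSubsystem.
; On BeginPlay it initializes a pool of BP_ExampleActor, then adds more actors of the same class.
; It binds handlers to the subsystem's spawn and return-to-pool delegates.
; Each handler prints the actor's name and location on screen, with the spawn message also showing its owner.
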(event Custom|Actor%20DeSpawned
  (params (Actor :type Actor%20Object%20Reference) (Transform :type Transform%20%28by%20ref%29))
  ;[1 1 1] Listen for actor Return To Pool function
  (Development|PrintString (Utilities|String|Append "Game Mode bound event saw that actor:" (Utilities|GetDisplayName Actor) " was DeSpawned at location" (Utilities|String|ToString(Vector) (.Location (Math|Transform|BreakTransform Transform)))) true true "(R=1.000000,G=0.969543,B=0.000000,A=1.000000)" 5.0))

(event Custom|Actor%20Spawned
  (params (Actor :type Actor%20Object%20Reference) (Transform :type Transform%20%28by%20ref%29))
  ;[1 1 1] Listen to spawn point "Broadcast Spawn"
  (Development|PrintString (Utilities|String|Append "Game Mode bound event saw that actor:" (Utilities|GetDisplayName Actor) " --- Owned by :" (Utilities|GetDisplayName (Components|GetOwner Actor)) "--- Spawned at location:" (Utilities|String|ToString(Vector) (.Location (Math|Transform|BreakTransform Transform)))) true true "(R=0.000000,G=0.660000,B=1.000000,A=1.000000)" 5.0))

(event EventBeginPlay
  ;[1 1 1] Start with some actors already in pool
  (Class|ActorPoolSubsystem|InitPool (Subsystems|GetActorPoolSubsystem) "/ActorPoolingSubsystem/BP_ExampleActor.BP_ExampleActor_C" 2)
  ;[1 1 1] Add some more actors (can be other types)
  (Class|ActorPoolSubsystem|AddActorsbyClass (Subsystems|GetActorPoolSubsystem) "/ActorPoolingSubsystem/BP_ExampleActor.BP_ExampleActor_C" 4)
  ;[1 1 1] Listen to spawn point "Broadcast Spawn"
  (EventDispatchers|BindEventtoOnActorSpawnDelegate (Subsystems|GetActorPoolSubsystem) (delegate Custom|Actor%20Spawned))
  ;[1 1 1] Listen for actor Return To Pool function
  (EventDispatchers|BindEventtoOnActorReturntoPoolDelegate (Subsystems|GetActorPoolSubsystem) (delegate Custom|Actor%20DeSpawned)))

(fn ConstructionScript)