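; Example actor for the Actor Pooling Subsystem that demonstrates the pool lifecycle callbacks by printing its name at each stage.
; BeginPlay runs only on first creation, while OnCreate fires on each spawn from the pool and returns the actor to the pool after a short delay.
; OnDestroy and the Enable and Disable Optimisations events only log, marking where custom cleanup and stored-state optimisations go.
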(event EventBeginPlay
  ;[1 1 1] Regular begin play (Do your heavy logic here, this wont be called by the pool when the actor is spawned, it will only run the first time this actor is created by the game)
  (Development|PrintString (Utilities|String|Append (Utilities|GetDisplayName self) ":: Begin Play") true true "(R=1.000000,G=0.065008,B=0.000000,A=1.000000)" 5.0))

(event EventPoolonDestroy
  ;[1 1 1] On Destroy (called when returning to pool)
  (Development|PrintString (Utilities|String|Append (Utilities|GetDisplayName self) ":: OnDestroy Called") true true "(R=1.000000,G=0.140704,B=0.991315,A=1.000000)" 5.0))

(event EventPoolEnableOptimisations
  ;[1 1 1] Set custom Optimisations when stored in pool
  (Development|PrintString (Utilities|String|Append (Utilities|GetDisplayName self) ":: Enable Optimisations Called") true true "(R=1.000000,G=0.953033,B=0.236324,A=1.000000)" 5.0))

(event EventPoolDisableOptimisations
  ;[1 1 1] Undo optimisations when spawned from pool
  (Development|PrintString (Utilities|String|Append (Utilities|GetDisplayName self) ":: Disable Optimisations Called") true true "(R=1.000000,G=0.953033,B=0.236324,A=1.000000)" 5.0))

(event EventPoolonCreate
  ;[1 1 1] OnCreate (called when spawned from pool)
  (Development|PrintString (Utilities|String|Append (Utilities|GetDisplayName self) ":: OnCreate called") true true "(R=1.000000,G=0.953033,B=0.236324,A=1.000000)" 5.0)
  (Utilities|FlowControl|Delay 2.9)
  ;[1 1 1] Return Actor to Pool
  (Class|ActorPoolSubsystem|ReturnActortoPool (Subsystems|GetActorPoolSubsystem) 0 true))

(fn ConstructionScript)