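; Example actor that demonstrates the lifecycle callbacks of an actor pool by printing its display name with each event.
; BeginPlay and the pool create, destroy, enable-optimization and disable-optimization events each print a message, with the optimization events serving as stubs for custom logic.
; After its create callback, the actor waits a few seconds, then returns to the pool through the ActorPoolSubsystem with broadcast enabled.
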(event EventBeginPlay
  (Development|PrintString (Utilities|String|Append (Utilities|GetDisplayName self) ":: Begin Play") true true "(R=1.000000,G=0.065008,B=0.000000,A=1.000000)" 5.0))

(event EventPoolEnableOptimizations
  ;[1 1 1] Set custom Optimizations when stored in pool
  (Development|PrintString (Utilities|String|Append (Utilities|GetDisplayName self) ":: Enable Optimisations Called") true true "(R=1.000000,G=0.953033,B=0.236324,A=1.000000)" 5.0))

(event EventPoolDisableOptimizations
  ;[1 1 1] Undo optimizations when spawned from pool
  (Development|PrintString (Utilities|String|Append (Utilities|GetDisplayName self) ":: Disable Optimisations Called") true true "(R=1.000000,G=0.953033,B=0.236324,A=1.000000)" 5.0))

(event EventPoolonCreate
  (Development|PrintString (Utilities|String|Append (Utilities|GetDisplayName self) ":: OnCreate called") true true "(R=1.000000,G=0.953033,B=0.236324,A=1.000000)" 5.0)
  (Utilities|FlowControl|Delay 2.9)
  ;[1 1 1] Return Actor to Pool
  (Class|ActorPoolSubsystem|ReturnActortoPool (Subsystems|GetActorPoolSubsystem) 0 true))

(event EventPoolonDestroy
  (Development|PrintString (Utilities|String|Append (Utilities|GetDisplayName self) ":: OnDestroy Called") true true "(R=1.000000,G=0.140704,B=0.991315,A=1.000000)" 5.0))

(fn ConstructionScript)